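; Enemy spawner for the bowling game that spawns queued enemy classes at its own location, facing the player.
; AddEnemyToList queues a class and spawns immediately if no VR player overlaps its sphere.
; Tick and a looping timer also drain the queue through SpawnEnemy, without that overlap check.
; It binds each enemy's death event and has a handler forwarding defeats to the Modo1 game mode; older random-navmesh spawn logic is disconnected.
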(event Custom|OnEnemyDefeated
  (bind _asmodo_1 (Utilities|Casting|CastToModo1 (Game|GetGameMode)))
  (Default|OnEnemyDefeated _asmodo_1))

(event Custom|TrySpawn
  (CallFunction|SpawnEnemy))

(event EventBeginPlay
  (Utilities|Time|SetTimerbyEvent (delegate Custom|TrySpawn) 2.0 true))

(event Collision|EventActorBeginOverlap
  (params (OtherActor :type Actor%20Object%20Reference)))

(event EventTick
  (params (DeltaSeconds :type Float%20%28single-precision%29))
  (CallFunction|SpawnEnemy))

(fn ConstructionScript)

(fn SpawnEnemy
  (bind _returnvalue (Transformation|GetActorTransform))
  (if (Utilities|Array|IsValidIndex (Variables|Default|GetEnemyList))
    (bind _returnvalue_2 (Game|SpawnActorfromClass (Utilities|Array|Get(acopy) (Variables|Default|GetEnemyList)) (Math|Transform|MakeTransform (.location _returnvalue) (Math|Rotator|FindLookatRotation (.location _returnvalue) (.location (Transformation|GetActorTransform (Game|Player|GetPlayerPawn 0)))) "1.000000,1.000000,1.000000") "Undefined" "MultiplyWithRoot" 0 0))
    (EventDispatchers|BindEventtoOnDeath _returnvalue_2 (EventDispatchers|CreateEvent :!event Custom|OnEnemyDefeated))
    (Development|PrintString "SPAWNEADO 
")
    (Utilities|Array|RemoveIndex (Variables|Default|GetEnemyList))
    (return true)
    (else
      (return false))))

(fn AddEnemytoList
  (params (Enemy :type BP%20CZ%20Bowl%20Class%20Reference%20%28by%20ref%29))
  (Utilities|Array|Add (Variables|Default|GetEnemyList) Enemy)
  (if (not (Utilities|Array|IsValidIndex (Collision|GetOverlappingActors (Variables|Default|GetSphere) "/Game/BOLERA/BluePrints/BP_PlayerVR.BP_PlayerVR_C" :!class /Script/Engine.PrimitiveComponent)))
    (CallFunction|SpawnEnemy)))