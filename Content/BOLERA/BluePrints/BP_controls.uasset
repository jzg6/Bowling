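; Control-hint display actor for the bowling area (BOLERA), labeling actions such as grab, hold, move, turn and special move.
; Each label is a child actor component holding a BP_SpawnSign.
; On BeginPlay it casts each child in sequence and sets its TEXT to the component's own object name, so component names double as displayed labels.
; A failed cast stops the remaining assignments.
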(event EventBeginPlay
  (bind _move (Variables|Default|GetMove))
  (bind _grab_right (Variables|Default|GetGrab%20Right))
  (bind _special_move__ (Variables|Default|GetSpecial%20Move%20!))
  (bind __ (Variables|Default|Get+))
  (bind _hold_left (Variables|Default|GetHold%20Left))
  (bind _grab_left (Variables|Default|GetGrab%20Left))
  (bind _turn_90º (Variables|Default|GetTurn%2090º))
  (bind _hold_right (Variables|Default|GetHold%20Right))
  ;[0.1148 0.004744 0.08581] PERDONAME DIOS
  (bind _asbp_spawn_sign (Utilities|Casting|CastToBP_SpawnSign (Variables|/Script/Engine.ChildActorComponent|GetChildActor _grab_left)))
  (Variables|/Game/BOLERA/BluePrints/Widgets/BP_SpawnSign.BP_SpawnSign_C|SetTEXT _asbp_spawn_sign (Utilities|GetObjectName _grab_left))
  (bind _asbp_spawn_sign_2 (Utilities|Casting|CastToBP_SpawnSign (Variables|/Script/Engine.ChildActorComponent|GetChildActor _hold_left)))
  (Variables|/Game/BOLERA/BluePrints/Widgets/BP_SpawnSign.BP_SpawnSign_C|SetTEXT _asbp_spawn_sign_2 (Utilities|GetObjectName _hold_left))
  (bind _asbp_spawn_sign_3 (Utilities|Casting|CastToBP_SpawnSign (Variables|/Script/Engine.ChildActorComponent|GetChildActor _move)))
  (Variables|/Game/BOLERA/BluePrints/Widgets/BP_SpawnSign.BP_SpawnSign_C|SetTEXT _asbp_spawn_sign_3 (Utilities|GetObjectName _move))
  (bind _asbp_spawn_sign_4 (Utilities|Casting|CastToBP_SpawnSign (Variables|/Script/Engine.ChildActorComponent|GetChildActor _turn_90º)))
  (Variables|/Game/BOLERA/BluePrints/Widgets/BP_SpawnSign.BP_SpawnSign_C|SetTEXT _asbp_spawn_sign_4 (Utilities|GetObjectName _turn_90º))
  (bind _asbp_spawn_sign_5 (Utilities|Casting|CastToBP_SpawnSign (Variables|/Script/Engine.ChildActorComponent|GetChildActor _hold_right)))
  (Variables|/Game/BOLERA/BluePrints/Widgets/BP_SpawnSign.BP_SpawnSign_C|SetTEXT _asbp_spawn_sign_5 (Utilities|GetObjectName _hold_right))
  (bind _asbp_spawn_sign_6 (Utilities|Casting|CastToBP_SpawnSign (Variables|/Script/Engine.ChildActorComponent|GetChildActor _grab_right)))
  (Variables|/Game/BOLERA/BluePrints/Widgets/BP_SpawnSign.BP_SpawnSign_C|SetTEXT _asbp_spawn_sign_6 (Utilities|GetObjectName _grab_right))
  (bind _asbp_spawn_sign_7 (Utilities|Casting|CastToBP_SpawnSign (Variables|/Script/Engine.ChildActorComponent|GetChildActor _special_move__)))
  (Variables|/Game/BOLERA/BluePrints/Widgets/BP_SpawnSign.BP_SpawnSign_C|SetTEXT _asbp_spawn_sign_7 (Utilities|GetObjectName _special_move__))
  (bind _asbp_spawn_sign_8 (Utilities|Casting|CastToBP_SpawnSign (Variables|/Script/Engine.ChildActorComponent|GetChildActor __)))
  (Variables|/Game/BOLERA/BluePrints/Widgets/BP_SpawnSign.BP_SpawnSign_C|SetTEXT _asbp_spawn_sign_8 (Utilities|GetObjectName __)))

(fn ConstructionScript)