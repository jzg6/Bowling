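; VR player pawn for the bowling game, with stick movement, 90-degree snap turning, object grabbing and ball launching.
; Enhanced Input adds camera-relative movement, which Tick consumes and applies without sweep.
; Grabbing line-traces for physics bodies and attaches hits to HeldObjectLocation; both grab inputs share this left-controller logic, so right-hand grabbing is unfinished.
; A button spawns BP_BowlingBall at the right controller and impulses it along actor forward.
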(event Custom|GrabObject
  (bind _motioncontrollerleft (Variables|Default|GetMotionControllerLeft))
  (bind _returnvalue (Transformation|GetWorldLocation _motioncontrollerleft))
  ;[0.238 0.2412 1] REHACER LAS FUNCIONES DE AGARRAR Y SOLTAR PARA QUE ACEPTEN PARAMETROS Y ASÍ SIRVAN PARA LAS DOS MANOS
  (bind (_outhit _returnvalue_2) (Collision|LineTraceForObjects _returnvalue (+ _returnvalue (* (Math|Vector|GetForwardVector _motioncontrollerleft) 10000)) (Utilities|Array|MakeArray "ObjectTypeQuery4") false 0 "ForDuration"))
  (if _returnvalue_2
    (Variables|Default|SetHitComponent (.HitComponent (Collision|BreakHitResult _outhit)))
    (if (Class|SceneComponent|IsAnySimulatingPhysics (.HitComponent (Collision|BreakHitResult _outhit)))
      (bind _output_get (Variables|Default|SetpickedActor (.HitActor (Collision|BreakHitResult _outhit))))
      (Physics|SetSimulatePhysics (.HitComponent (Collision|BreakHitResult _outhit)) false)
      (Transformation|AttachComponentToComponent _output_get (Variables|Default|GetHeldObjectLocation) "None" "SnapToTarget" "SnapToTarget" "KeepWorld" true)
      (Variables|Default|SetisHoldingObjectL true))))

(event Custom|ReleaseObject
  ;[0.238 0.2412 1] REHACER LAS FUNCIONES DE AGARRAR Y SOLTAR PARA QUE ACEPTEN PARAMETROS Y ASÍ SIRVAN PARA LAS DOS MANOS
  (Utilities|IsValid (Variables|Default|GetpickedActor)
    (:Is%20Valid
      (Transformation|DetachFromActor (Variables|Default|GetpickedActor) "KeepWorld" "KeepWorld" "KeepWorld")
      (Utilities|IsValid 0
        (:Is%20Valid
          (Physics|SetSimulatePhysics (Variables|Default|GetHitComponent) true)
          (Variables|Default|SetisHoldingObjectL false)
          (Variables|Default|SetpickedActor 0)
          (Variables|Default|SetHitComponent 0))))))

(event Input|EnhancedActionEvents|EnhancedInputActionIA_GrabLeft
  (params (ActionValue :type Boolean) (ElapsedSeconds :type Float%20%28double-precision%29) (TriggeredSeconds :type Float%20%28double-precision%29) (InputAction :type Input%20Action%20Object%20Reference :default "/Game/BOLERA/Input/IA_GrabLeft.IA_GrabLeft"))
  ;[0.238 0.2412 1] REHACER LAS FUNCIONES DE AGARRAR Y SOLTAR PARA QUE ACEPTEN PARAMETROS Y ASÍ SIRVAN PARA LAS DOS MANOS
  (if ActionValue
    (if (not (Variables|Default|GetisHoldingObjectL))
      (CallFunction|GrabObject))
    (else
      (CallFunction|ReleaseObject))))

(event Input|EnhancedActionEvents|EnhancedInputActionIA_GrabRight
  (params (ActionValue :type Boolean) (ElapsedSeconds :type Float%20%28double-precision%29) (TriggeredSeconds :type Float%20%28double-precision%29) (InputAction :type Input%20Action%20Object%20Reference :default "/Game/BOLERA/Input/IA_GrabRight.IA_GrabRight"))
  ;[0.238 0.2412 1] REHACER LAS FUNCIONES DE AGARRAR Y SOLTAR PARA QUE ACEPTEN PARAMETROS Y ASÍ SIRVAN PARA LAS DOS MANOS
  (if ActionValue
    (if (not (Variables|Default|GetisHoldingObjectR))
      (CallFunction|GrabObject))
    (else
      (CallFunction|ReleaseObject))))

(event Input|EnhancedActionEvents|EnhancedInputActionIA_HOLA
  (params (ActionValue :type Boolean) (ElapsedSeconds :type Float%20%28double-precision%29) (TriggeredSeconds :type Float%20%28double-precision%29) (InputAction :type Input%20Action%20Object%20Reference :default "/Game/BOLERA/Input/IA_HOLA.IA_HOLA"))
  (Development|PrintString "Hello"))

(event Input|EnhancedActionEvents|EnhancedInputActionIA_GrabLeft
  (params (ActionValue :type Boolean) (ElapsedSeconds :type Float%20%28double-precision%29) (TriggeredSeconds :type Float%20%28double-precision%29) (InputAction :type Input%20Action%20Object%20Reference :default "/Game/BOLERA/Input/IA_GrabLeft.IA_GrabLeft"))
  (Development|PrintString "TRIGGER"))

(event Input|EnhancedActionEvents|EnhancedInputActionIA_TURN
  (params (ActionValue :type Float%20%28double-precision%29) (ElapsedSeconds :type Float%20%28double-precision%29) (TriggeredSeconds :type Float%20%28double-precision%29) (InputAction :type Input%20Action%20Object%20Reference :default "/Game/BOLERA/Input/IA_TURN.IA_TURN"))
  (:Started
    (if (> ActionValue 0.0)
      (Class|Actor|AddActorWorldRotation (Math|Rotator|MakeRotator 0.0 0.0 9e+01))
      (else
        (Class|Actor|AddActorWorldRotation (Math|Rotator|MakeRotator 0.0 0.0 -9e+01))))))

(event Input|EnhancedActionEvents|EnhancedInputActionIA_MOVE
  (params (ActionValue :type Vector%202D%20Structure) (ElapsedSeconds :type Float%20%28double-precision%29) (TriggeredSeconds :type Float%20%28double-precision%29) (InputAction :type Input%20Action%20Object%20Reference :default "/Game/BOLERA/Input/IA_MOVE.IA_MOVE"))
  (bind _camera (Variables|Default|GetCamera))
  (bind _returnvalue (Math|Vector|GetForwardVector _camera))
  (bind _returnvalue_2 (Math|Vector|GetRightVector _camera))
  (bind _returnvalue_3 (* (.y ActionValue) _returnvalue))
  (bind _returnvalue_4 (* (.x ActionValue) _returnvalue_2))
  (bind _returnvalue_5 (+ _returnvalue_4 _returnvalue_3))
  (Pawn|Input|AddMovementInput (Math|Vector|MakeVector (.x _returnvalue_5) (.y _returnvalue_5) 0.0) 1e+01 false)
  (Development|PrintString "MOVER"))

(event Input|EnhancedActionEvents|EnhancedInputActionIA_BOTON
  (params (ActionValue :type Boolean) (ElapsedSeconds :type Float%20%28double-precision%29) (TriggeredSeconds :type Float%20%28double-precision%29) (InputAction :type Input%20Action%20Object%20Reference :default "/Game/BOLERA/Input/IA_BOTON.IA_BOTON"))
  (:Started
    (bind _returnvalue (Game|SpawnActorfromClass "/Game/BOLERA/BluePrints/BP_BowlingBall.BP_BowlingBall_C" (Transformation|GetWorldTransform (Variables|Default|GetMotionControllerRight)) "Undefined" "MultiplyWithRoot" 0 0))
    (Physics|AddImpulse (Variables|/Game/BOLERA/BluePrints/BP_BowlingBall.BP_BowlingBall_C|GetSphere _returnvalue) (* (Transformation|GetActorForwardVector) "10000.000000,10000.000000,10000.000000") "None" false)))

(event EventBeginPlay
  (if (Class|HeadMountedDisplayFunctionLibrary|IsHeadMountedDisplayEnabled)
    (Class|HeadMountedDisplayFunctionLibrary|SetTrackingOrigin "Stage"))
  (bind _asplayer_controller (Utilities|Casting|CastToPlayerController (Pawn|GetController)))
  (Utilities|IsValid (PlayerController|LocalPlayerSubsystems|GetEnhancedInputLocalPlayerSubsystem _asplayer_controller)
    (:Is%20Valid
      (Input|AddMappingContext (PlayerController|LocalPlayerSubsystems|GetEnhancedInputLocalPlayerSubsystem _asplayer_controller) "/Game/BOLERA/Input/inputs.inputs" 0 "(bIgnoreAllPressedKeysUntilRelease=True,bForceImmediately=False,bNotifyUserSettings=False)"))))

(event Collision|EventActorBeginOverlap
  (params (OtherActor :type Actor%20Object%20Reference)))

(event EventTick
  (params (DeltaSeconds :type Float%20%28single-precision%29))
  (bind _returnvalue (Class|Pawn|ConsumeMovementInputVector))
  (Transformation|SetActorLocation (+ _returnvalue (Transformation|GetActorLocation)) false false))

(fn ConstructionScript)