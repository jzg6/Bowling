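; BP_CZBowl is an AI enemy that wanders the navmesh, chases the player on sight, and ends the Modo1 game when its capsule overlaps the VR pawn.
; Tick drives delayed random wandering, and PawnSensing switches it to pursuit.
; A hit from a bowling ball, BP_Bowl or dead BP_CZBowl kills it, allowing chain reactions.
; Death plays audio and launches it backward and upward, spinning until it fires OnDeath and destroys itself.
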(event OnSeePawn(PawnSensing)
  (params (Pawn :type Pawn%20Object%20Reference))
  (if (Variables|Default|Getdead)
    (Variables|Default|SetplayerInSight false)
    (else
      (AI|AIMoveTo self "0, 0, 0" (Game|Player|GetPlayerPawn 0) 0.0 false
        (:then
          (Variables|Default|SetplayerInSight true))))))

(event OnComponentBeginOverlap(CapsuleComponent)
  (params (OverlappedComponent :type Primitive%20Component%20Object%20Reference) (OtherActor :type Actor%20Object%20Reference) (OtherComp :type Primitive%20Component%20Object%20Reference) (OtherBodyIndex :type Integer) (bFromSweep :type Boolean) (SweepResult :type Hit%20Result%20Structure%20%28by%20ref%29))
  (Utilities|Casting|CastToBP_VRPawn2 OtherActor)
  (Development|PrintString "Se acabó para ti" false false)
  (bind _asmodo_1 (Utilities|Casting|CastToModo1 (Game|GetGameMode)))
  (Default|SetEndGame _asmodo_1))

(event EventBeginPlay)

(event Collision|EventActorBeginOverlap
  (params (OtherActor :type Actor%20Object%20Reference)))

(event EventTick
  (params (DeltaSeconds :type Float%20%28single-precision%29))
  (if (Variables|Default|Getdead)
    (Transformation|AddActorLocalRotation "2.000000,2.000000,2.000000" false false)
    (Utilities|FlowControl|Delay 1.5)
    (Default|CallOnDeath)
    (Utilities|IsValid self
      (:Is%20Valid
        (Actor|DestroyActor)))
    (elif (not (Variables|Default|GetplayerInSight))
      (bind _randomlocation (Class|NavigationSystemV1|GetRandomLocationinNavigableRadius (.location (Transformation|GetActorTransform)) 1e+04 0 0))
      (Utilities|FlowControl|Delay 3.0)
      (AI|AIMoveTo self _randomlocation 0 5.0 false))))

(event Collision|EventHit
  (params (MyComp :type Primitive%20Component%20Object%20Reference) (Other :type Actor%20Object%20Reference) (OtherComp :type Primitive%20Component%20Object%20Reference) (bSelfMoved :type Boolean) (HitLocation :type Vector :default "0, 0, 0") (HitNormal :type Vector :default "0, 0, 0") (NormalImpulse :type Vector :default "0, 0, 0") (Hit :type Hit%20Result%20Structure%20%28by%20ref%29))
  (bind _charactermovement (Variables|Character|GetCharacterMovement))
  (if (not (Variables|Default|Getdead))
    (Utilities|Casting|CastToBP_BowlingBall Other
      (:then
        (Variables|Default|Setdead true :!label _label)
        (Audio|Components|Audio|Play (Variables|Default|GetAudio) 0.0)
        (AI|Navigation|StopMovement (AI|GetAIController self))
        (Physics|AddImpulse _charactermovement (* (Math|Vector|NegateVector (Transformation|GetActorForwardVector)) "900000.000000,900000.000000,900000.000000") false)
        (Physics|AddImpulse _charactermovement "0.000000,0.000000,99990.000000" false))
      (:CastFailed
        (Utilities|Casting|CastToBP_Bowl Other
          (:then
            (goto _label))
          (:CastFailed
            (bind _asbp_czbowl (Utilities|Casting|CastToBP_CZBowl Other))
            (if (Variables|BP_CZBowl_C|Getdead _asbp_czbowl)
              (goto _label))))))))

(fn ConstructionScript)