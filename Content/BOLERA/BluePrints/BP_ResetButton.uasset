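; BP_ResetButton is a reset trigger in the bowling (BOLERA) content that respawns the set of bowls.
; Any overlap with its Box destroys every valid actor in Bowls, then spawns a BP_Bowl slightly above each Spawns actor, using its rotation and BowlSize scale.
; New bowls are inserted into Bowls without clearing old entries, and Audio plays on each spawn iteration.
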(event OnComponentBeginOverlap(Box)
  (params (OverlappedComponent :type Primitive%20Component%20Object%20Reference) (OtherActor :type Actor%20Object%20Reference) (OtherComp :type Primitive%20Component%20Object%20Reference) (OtherBodyIndex :type Integer) (bFromSweep :type Boolean) (SweepResult :type Hit%20Result%20Structure%20%28by%20ref%29))
  (for _array_element (Variables|Default|GetBowls)
    (Utilities|IsValid _array_element
      (:Is%20Valid
        (Actor|DestroyActor _array_element))))
  (for (_array_element_2 _array_index) (Variables|Default|GetSpawns)
    (bind _returnvalue (Game|SpawnActorfromClass "/Game/BOLERA/BluePrints/BP_Bowl.BP_Bowl_C" (Math|Transform|MakeTransform (+ (.location (Transformation|GetActorTransform _array_element_2)) "0.000000,0.000000,1.000000") (.rotation (Transformation|GetActorTransform _array_element_2)) (Variables|Default|GetbowlSize)) "Undefined" "MultiplyWithRoot" 0 0))
    (Utilities|Array|Insert (Variables|Default|GetBowls) _returnvalue _array_index)
    (Audio|Components|Audio|Play (Variables|Default|GetAudio) 0.0)))

(event EventBeginPlay)

(event Collision|EventActorBeginOverlap
  (params (OtherActor :type Actor%20Object%20Reference)))

(event EventTick
  (params (DeltaSeconds :type Float%20%28single-precision%29)))

(fn ConstructionScript)